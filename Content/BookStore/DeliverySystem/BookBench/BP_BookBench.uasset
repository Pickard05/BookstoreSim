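; Book bench in the book store delivery system where the player places a box on a platform and raises it.
; Interact either snaps the player's held box onto the bench or, from the panel zone, plays a timeline lifting the platform and scaling its cylinder.
; An overlap volume tracks box presence, using a delayed gate for exit.
; The panel zone runs a looping timer that refreshes the player's contextual prompt.
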(event `self.ReceiveBeginPlay`
  (set `self.PlatformStart Location` (`SceneComponent.RelativeLocation` (`self.PlatformRaise`)))
  (set `self.CylinderStartScale` (`SceneComponent.RelativeScale3D` (`self.PlatformCylinder`)))
  (bind _asbp_first_person_character (cast `/Game/FirstPerson/Blueprints/BP_FirstPersonCharacter` (`GameplayStatics.GetPlayerCharacter` 0)))
  (set `self.As BP First Person Character` _asbp_first_person_character))

(event `self.Platform Box Detection.OnComponentBeginOverlap`
  (params (OverlappedComponent :type "PrimitiveComponent Object Reference") (OtherActor :type "Actor Object Reference") (OtherComp :type "PrimitiveComponent Object Reference") (OtherBodyIndex :type Integer) (bFromSweep :type Boolean) (SweepResult :type "HitResult Structure (by ref)"))
  (if (`KismetSystemLibrary.DoesImplementInterface` OtherActor "/Game/BookStore/DeliverySystem/BookBox/BPI_BoxInterface.BPI_BoxInterface_C")
    (set `self.Box on Platform` true)
    (`KismetSystemLibrary.Delay` 1.0)
    (goto _label :!via `Open`)))

(event `self.Platform Box Detection.OnComponentEndOverlap`
  (params (OverlappedComponent :type "PrimitiveComponent Object Reference") (OtherActor :type "Actor Object Reference") (OtherComp :type "PrimitiveComponent Object Reference") (OtherBodyIndex :type Integer))
  (`/Engine/EditorBlueprintResources/StandardMacros.Gate` true :!label _label
    (:`Exit`
      (if (`KismetSystemLibrary.DoesImplementInterface` OtherActor "/Game/BookStore/DeliverySystem/BookBox/BPI_BoxInterface.BPI_BoxInterface_C")
        (set `self.Box on Platform` false)
        (goto _label :!via `Close`)))))

(event `interact text check`
  (bind _as_bp_first_person_character (`self.As BP First Person Character`))
  (bind _interacttext (`/Game/BookStore/Widgets/WB_Interact.interacttext` (`/Game/FirstPerson/Blueprints/BP_FirstPersonCharacter.interact text` _as_bp_first_person_character)))
  (`/Engine/EditorBlueprintResources/StandardMacros.IsValid` (`/Game/FirstPerson/Blueprints/BP_FirstPersonCharacter.Active Box` _as_bp_first_person_character)
    (:`Is Valid`
      (`TextBlock.SetText` _interacttext "Press F to place the box"))
    (:`Is Not Valid`
      (if (`self.Box on Platform`)
        (`TextBlock.SetText` _interacttext "Press E to Raise Platform")
        (else
          (`TextBlock.SetText` _interacttext "Place a box on the Platform"))))))

(event `Raise Platform`
  (bind (_platformstart_location_x _platformstart_location_y _platformstart_location_z) (`KismetMathLibrary.BreakVector` (`self.PlatformStart Location`)))
  ; Raise / lower Platform
  (if (`self.Box on Platform`)
    (bind (_direction _raise_lower_time _cylinderscale) (`Timeline|Raise / Lower Platform` :!via `PlayFromStart` :!label _label_2)
      (:`Update`
        (`SceneComponent.K2_SetRelativeLocation` (`self.PlatformRaise`) (`KismetMathLibrary.MakeVector` _platformstart_location_x _platformstart_location_y (`KismetMathLibrary.Lerp` _platformstart_location_z 50.0 _raise_lower_time)) false false)
        (`SceneComponent.SetRelativeScale3D` (`self.PlatformCylinder`) (`KismetMathLibrary.VLerp` (`self.CylinderStartScale`) _cylinderscale _raise_lower_time))))
    (else
      (goto _label_2 :!via `Reverse`))))

(event `start time`
  (bind _returnvalue (`KismetSystemLibrary.K2_SetTimerDelegate` (delegate `interact text check`) 0.1 true))
  (set `self.interact timer` _returnvalue))

(event `/Game/FirstPerson/Blueprints/BPI_Interact_Interface.Interact`
  (params (Interactor :type "/Game/FirstPerson/Blueprints/BP_FirstPersonCharacter Object Reference"))
  (bind _box_platformscene (`self.Box PlatformScene`))
  (if (`self.Box on Platform`)
    (if (`self.canRaise_lower`)
      (`self.Raise Platform`))
    (else
      (`/Game/FirstPerson/Blueprints/BP_FirstPersonCharacter.detatch box` Interactor (`SceneComponent.K2_GetComponentLocation` _box_platformscene) (`SceneComponent.K2_GetComponentRotation` _box_platformscene))
      (bind _active_box (`/Game/FirstPerson/Blueprints/BP_FirstPersonCharacter.Active Box` Interactor)
        (:`then`
          (`self.K2_AttachToComponent` _active_box (`self.Box PlatformScene`) "None" "SnapToTarget" "SnapToTarget" "KeepRelative" true)
          (set `/Game/BookStore/DeliverySystem/BookBox/BP_BookBoxMaster.onBench?` true _active_box)
          (set `/Game/FirstPerson/Blueprints/BP_FirstPersonCharacter.Active Box` null Interactor))
        (:`else`)))))

(event `self.Panel Detection.OnComponentBeginOverlap`
  (params (OverlappedComponent :type "PrimitiveComponent Object Reference") (OtherActor :type "Actor Object Reference") (OtherComp :type "PrimitiveComponent Object Reference") (OtherBodyIndex :type Integer) (bFromSweep :type Boolean) (SweepResult :type "HitResult Structure (by ref)"))
  (if (== OtherActor (`GameplayStatics.GetPlayerCharacter` 0))
    (`self.start time`)
    (`Widget.SetVisibility` (`/Game/BookStore/Widgets/WB_Interact.interacttext` (`/Game/FirstPerson/Blueprints/BP_FirstPersonCharacter.interact text` (`self.As BP First Person Character`))) "SelfHitTestInvisible")
    (if (`self.Box on Platform`)
      (set `self.canRaise_lower` true))))

(event `self.Panel Detection.OnComponentEndOverlap`
  (params (OverlappedComponent :type "PrimitiveComponent Object Reference") (OtherActor :type "Actor Object Reference") (OtherComp :type "PrimitiveComponent Object Reference") (OtherBodyIndex :type Integer))
  (if (== OtherActor (`GameplayStatics.GetPlayerCharacter` 0))
    (set `self.canRaise_lower` false)
    (`Widget.SetVisibility` (`/Game/BookStore/Widgets/WB_Interact.interacttext` (`/Game/FirstPerson/Blueprints/BP_FirstPersonCharacter.interact text` (`self.As BP First Person Character`))) "Collapsed")
    (`KismetSystemLibrary.K2_ClearAndInvalidateTimerHandle` (`self.interact timer`))))

(fn `UserConstructionScript`)