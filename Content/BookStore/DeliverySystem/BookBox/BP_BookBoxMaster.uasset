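; Delivery book box the player picks up, drops with brief physics, and unpacks on a bench.
; Interact toggles carrying off the bench; on it, removes the tape, then toggles the timeline-animated lid.
; Tape removal starts a looping timer that spawns weighted-random books at successive spawn points, re-rolling the 3–5 limit each tick.
; A sphere overlap shows a pick-up/drop prompt, refreshed by timer.
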(event `self.ReceiveBeginPlay`
  (set `self.Active Spawn Point` (`self.SpawnPoint1`))
  (bind _asbp_first_person_character (cast `/Game/FirstPerson/Blueprints/BP_FirstPersonCharacter` (`GameplayStatics.GetPlayerCharacter` 0)))
  (set `self.As BP First Person Character` _asbp_first_person_character))

(event `Spawn Event`
  ; Book Spawn / Might Change or improve
  (bind _returnvalue (`KismetSystemLibrary.K2_SetTimerDelegate` (delegate `Spawn 5 Books`) 0.1 true))
  (set `self.Small Book Timer` _returnvalue))

(event `Spawn 5 Books`
  (bind _spawn_point_array (`self.Spawn Point Array`))
  ; Book Spawn / Might Change or improve
  (`self.BookToSpawn`)
  (if (>= (`self.Spawn Count`) (`self.SpawnCountMax`))
    (`KismetSystemLibrary.K2_PauseTimerHandle` (`self.Small Book Timer`))
    (else
      (bind _returnvalue (`|SpawnActorFromClass` (`self.BookClass`) (`KismetMathLibrary.MakeTransform` (`SceneComponent.K2_GetComponentLocation` (`self.Active Spawn Point`)) (`self.Spawn Transform Rotation`)) "AlwaysSpawn" "MultiplyWithRoot" null null))
      (`/Engine/EditorBlueprintResources/StandardMacros.IncrementInt` (`self.Spawn Count`)
        (:`  `
          (`KismetArrayLibrary.Array_Add` (`self.BookSpawnedArray`) _returnvalue)
          (`KismetArrayLibrary.Array_RemoveItem` _spawn_point_array (`|GetArrayItem` _spawn_point_array))
          (set `self.Active Spawn Point` (`|GetArrayItem` _spawn_point_array)))))))

(event `/Game/BookStore/DeliverySystem/BookBox/BPI_BoxInterface.OpenBox`
  ; Open/Close Lid
  (if (not (`self.InMotion?`))
    (`/Engine/EditorBlueprintResources/StandardMacros.FlipFlop`
      (:`A`
        (set `self.InMotion?` true)
        (bind (_direction _open_close_lid) (`Timeline|Open` :!via `PlayFromStart` :!label _label)
          (:`Update`
            (`SceneComponent.K2_SetRelativeRotation` (`self.lidleft`) (`KismetMathLibrary.RLerp` (struct :`Pitch` 180.0 :`Yaw` 180.0 :`Roll` 180.0) (struct :`Pitch` 70.0 :`Yaw` 180.0 :`Roll` 180.0) _open_close_lid true) false false)
            (`SceneComponent.K2_SetRelativeRotation` (`self.lidright`) (`KismetMathLibrary.RLerp` (struct :`Yaw` 180.0) (struct :`Pitch` 120.0 :`Yaw` 180.0) _open_close_lid true) false false))
          (:`Finished`
            (set `self.InMotion?` false))))
      (:`B`
        (set `self.InMotion?` true)
        (goto _label :!via `Reverse`)))))

(event `/Game/FirstPerson/Blueprints/BPI_Interact_Interface.Interact`
  (params (Interactor :type "/Game/FirstPerson/Blueprints/BP_FirstPersonCharacter Object Reference"))
  ; Hold Box
  (if (`self.onBench?`)
    (if (`self.Tape Removed?`)
      (`/Game/BookStore/DeliverySystem/BookBox/BPI_BoxInterface.OpenBox`)
      (set `self.boxOpenn` true)
      (else
        (`/Game/BookStore/DeliverySystem/BookBox/BPI_BoxInterface.RemoveTape`)
        (set `self.InMotion?` false)))
    (else
      (`/Engine/EditorBlueprintResources/StandardMacros.IsValid` (`/Game/FirstPerson/Blueprints/BP_FirstPersonCharacter.Active Box` Interactor)
        (:`Is Valid`
          (`/Game/FirstPerson/Blueprints/BP_FirstPersonCharacter.Detach Current Box` Interactor)
          (set `/Game/FirstPerson/Blueprints/BP_FirstPersonCharacter.Is GrabbingbOX` false Interactor)
          (set `self.InMotion?` false)
          (set `/Game/FirstPerson/Blueprints/BP_FirstPersonCharacter.Active Box` null Interactor)
          (`PrimitiveComponent.SetSimulatePhysics` (`self.Front`) true)
          (`KismetSystemLibrary.Delay` 2.0)
          (`PrimitiveComponent.SetSimulatePhysics` (`self.Front`) false))
        (:`Is Not Valid`
          (if (not (`SceneComponent.IsSimulatingPhysics` (`self.Front`) "None"))
            (`self.Attach Box to Player` (`/Game/FirstPerson/Blueprints/BP_FirstPersonCharacter.FirstPersonMesh` Interactor) "Box_Socket2")
            (set `self.InMotion?` true)
            (set `/Game/FirstPerson/Blueprints/BP_FirstPersonCharacter.Is GrabbingbOX` true Interactor)
            (set `/Game/FirstPerson/Blueprints/BP_FirstPersonCharacter.Active Box` self Interactor)))))))

(event `/Game/BookStore/DeliverySystem/BookBox/BPI_BoxInterface.RemoveTape`
  (bind _tape (`self.Tape`))
  (bind (_relativescale3d_x _relativescale3d_y _relativescale3d_z) (`KismetMathLibrary.BreakVector` (`SceneComponent.RelativeScale3D` _tape)))
  ; Remove Tape
  (if (`self.onBench?`)
    (`/Engine/EditorBlueprintResources/StandardMacros.DoOnce` false
      (:`Completed`
        (`self.Spawn Event`)
        (bind (_direction _remove_tape) (`Timeline|Remove Tape` :!via `PlayFromStart`)
          (:`Update`
            (`SceneComponent.SetRelativeScale3D` _tape (`KismetMathLibrary.MakeVector` _relativescale3d_x (`KismetMathLibrary.Lerp` _relativescale3d_y 0.0 _remove_tape) _relativescale3d_z))
            (set `self.Tape Removed?` true)))))))

(event `Attach Box to Player`
  (params (Parent :type "SceneComponent Object Reference") (SocketName :type Name))
  ; Hold Box
  (`self.K2_AttachToComponent` Parent SocketName "SnapToTarget" "SnapToTarget" "SnapToTarget"))

(event `self.Sphere.OnComponentBeginOverlap`
  (params (OverlappedComponent :type "PrimitiveComponent Object Reference") (OtherActor :type "Actor Object Reference") (OtherComp :type "PrimitiveComponent Object Reference") (OtherBodyIndex :type Integer) (bFromSweep :type Boolean) (SweepResult :type "HitResult Structure (by ref)"))
  (if (== OtherActor (`self.As BP First Person Character`))
    (`Widget.SetVisibility` (`/Game/BookStore/Widgets/WB_Interact.interacttext` (`/Game/FirstPerson/Blueprints/BP_FirstPersonCharacter.interact text` (`self.As BP First Person Character`))) "HitTestInvisible")
    (`self.timer interact`)))

(event `timer interact`
  (bind _returnvalue (`KismetSystemLibrary.K2_SetTimerDelegate` (delegate `interact timer`) 0.1 true))
  (set `self.interact time handle` _returnvalue))

(event `interact timer`
  (bind _as_bp_first_person_character (`self.As BP First Person Character`))
  (bind _interacttext (`/Game/BookStore/Widgets/WB_Interact.interacttext` (`/Game/FirstPerson/Blueprints/BP_FirstPersonCharacter.interact text` _as_bp_first_person_character)))
  (`/Game/FirstPerson/Blueprints/BP_FirstPersonCharacter.Active Box` _as_bp_first_person_character
    (:`then`
      ; Hold Box
      (`TextBlock.SetText` _interacttext "Press E to drop Box"))
    (:`else`
      (`TextBlock.SetText` _interacttext "Press E to pick up"))))

(event `self.Sphere.OnComponentEndOverlap`
  (params (OverlappedComponent :type "PrimitiveComponent Object Reference") (OtherActor :type "Actor Object Reference") (OtherComp :type "PrimitiveComponent Object Reference") (OtherBodyIndex :type Integer))
  (bind _interacttext (`/Game/BookStore/Widgets/WB_Interact.interacttext` (`/Game/FirstPerson/Blueprints/BP_FirstPersonCharacter.interact text` (`self.As BP First Person Character`))))
  (if (== OtherActor (`self.As BP First Person Character`))
    (`Widget.SetVisibility` _interacttext "Collapsed")
    (`TextBlock.SetText` _interacttext "")
    (`KismetSystemLibrary.K2_ClearAndInvalidateTimerHandle` (`self.interact time handle`))))

(fn `BookToSpawn`
  (set `self.SpawnCountMax` (`KismetMathLibrary.RandomIntegerInRange` 3 5))
  (bind _output_get (set `self.Spawn Rate Int` (`KismetMathLibrary.RandomIntegerInRange` 0 150)))
  (`KismetSystemLibrary.PrintString` (`KismetStringLibrary.Conv_IntToString` _output_get))
  (if (<= (`self.Spawn Rate Int`) 70)
    (set `self.BookClass` (`|GetArrayItem` (`self.BookClassArray`)))
    (elif (<= (`self.Spawn Rate Int`) 110)
      (set `self.BookClass` (`|GetArrayItem` (`self.BookClassArray`) 1))
      (elif (<= (`self.Spawn Rate Int`) 130)
        (set `self.BookClass` (`|GetArrayItem` (`self.BookClassArray`) 2))
        (elif (<= (`self.Spawn Rate Int`) 145)
          (set `self.BookClass` (`|GetArrayItem` (`self.BookClassArray`) 3))
          (elif (>= (`self.Spawn Rate Int`) 149)
            (set `self.BookClass` (`|GetArrayItem` (`self.BookClassArray`) 4))))))))

(fn `UserConstructionScript`
  (bind _spawn_point_array (`self.Spawn Point Array`))
  (`KismetArrayLibrary.Array_Add` _spawn_point_array (`self.SpawnPoint1`))
  (`KismetArrayLibrary.Array_Add` _spawn_point_array (`self.SpawnPoint2`))
  (`KismetArrayLibrary.Array_Add` _spawn_point_array (`self.SpawnPoint3`))
  (`KismetArrayLibrary.Array_Add` _spawn_point_array (`self.SpawnPoint4`))
  (`KismetArrayLibrary.Array_Add` _spawn_point_array (`self.SpawnPoint5`)))