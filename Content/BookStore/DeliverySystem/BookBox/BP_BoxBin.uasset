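; BP_BoxBin is an interactable bin where the player disposes of empty book boxes in the bookstore delivery system.
; On Interact, it clears the player's grab state, destroys a held empty box and spawns a BP_foldedBox at EmptyBoxSpawn.
; Folded boxes are tracked in an array that flags the bin full at ten.
; A full bin only prints messages, with no emptying logic in this graph.
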(event `self.ReceiveBeginPlay`
  (bind _asbp_first_person_character (cast `/Game/FirstPerson/Blueprints/BP_FirstPersonCharacter` (`GameplayStatics.GetPlayerCharacter` 0)))
  (set `self.As BP First Person Character` _asbp_first_person_character))

(event `/Game/FirstPerson/Blueprints/BPI_Interact_Interface.Interact`
  (params (Interactor :type "/Game/FirstPerson/Blueprints/BP_FirstPersonCharacter Object Reference"))
  (bind _empty_box_array (`self.Empty box array`))
  (bind _as_bp_first_person_character (`self.As BP First Person Character`))
  (bind (_returnvalue_location _returnvalue_rotation) (`KismetMathLibrary.BreakTransform` (`SceneComponent.K2_GetComponentToWorld` (`self.empty box spawn`))))
  (if (`self.Full`)
    (`/Game/FirstPerson/Blueprints/BP_FirstPersonCharacter.Active Box` Interactor
      (:`then`
        (`KismetSystemLibrary.PrintString` "The bin needs emptying"))
      (:`else`
        (`KismetSystemLibrary.PrintString` "Empty Bin")))
    (else
      (bind _active_box (`/Game/FirstPerson/Blueprints/BP_FirstPersonCharacter.Active Box` Interactor)
        (:`then`
          (bind _output_get (set `self.empty box` _active_box))
          (if (`/Game/BookStore/DeliverySystem/BookBox/BP_BookBoxMaster.BoxEmpty?` _output_get)
            (set `/Game/FirstPerson/Blueprints/BP_FirstPersonCharacter.Is GrabbingbOX` false _as_bp_first_person_character)
            (`self.SetActorHiddenInGame` _active_box true)
            (set `/Game/FirstPerson/Blueprints/BP_FirstPersonCharacter.Active Box` null _as_bp_first_person_character)
            (`self.K2_DestroyActor` (`self.empty box`))
            (bind _returnvalue (`|SpawnActorFromClass` "/Game/BookStore/DeliverySystem/BookBox/BP_foldedBox.BP_foldedBox_C" (`KismetMathLibrary.MakeTransform` _returnvalue_location _returnvalue_rotation) "Undefined" "MultiplyWithRoot" null null))
            (`KismetArrayLibrary.Array_Add` _empty_box_array _returnvalue)
            (if (== (`KismetArrayLibrary.Array_Length` _empty_box_array) 10)
              (set `self.Full` true)
              (else
                (set `self.Full` false)))))
        (:`else`)))))

(fn `UserConstructionScript`)