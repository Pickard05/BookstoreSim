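; BP_Book_Common is a common book actor for the book store that randomizes its identity and appearance at BeginPlay.
; It picks a random row from the DT_CommonBooks data table and stores it as CommonBookStats.
; From that row it randomly chooses a small, medium or large scale and one of the listed meshes for BookMesh.
; The construction script only calls the parent's.
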(event `self.ReceiveBeginPlay`
  ; Set Random Common Book
  (bind _outrownames (`DataTableFunctionLibrary.GetDataTableRowNames` "/Game/BookStore/Data/CommonBooks/DT_CommonBooks.DT_CommonBooks"))
  (bind _returnvalue (`|GetDataTableRow` "/Game/BookStore/Data/CommonBooks/DT_CommonBooks.DT_CommonBooks" (`KismetArrayLibrary.Array_Random` _outrownames))
    (:`then`
      (bind _output_get (set `self.Common book stats` _returnvalue))
      (bind ((`Mesh_27_752171AE409F7781408030BB14012CC1` _mesh) (`SmallBookSize_25_F9480B5A4975899F018DF7A804B5BB63` _smallbooksize) (`MediumBookSize_24_CAF9D2E5485E5E9A761ED4899B835688` _mediumbooksize) (`LargeBookSize_26_BF94ECEC4DB3EB3FD7B317BBF2BCFB57` _largebooksize)) (break `/Game/BookStore/Data/CommonBooks/S_CommonBooks` _output_get))
      ; replace with book mesh
      (`SceneComponent.SetRelativeScale3D` (`self.BookMesh`) (`KismetArrayLibrary.Array_Random` (`|MakeArray` _smallbooksize _mediumbooksize _largebooksize)))
      (`StaticMeshComponent.SetStaticMesh` (`self.BookMesh`) (`KismetArrayLibrary.Array_Random` _mesh)))))

(fn `UserConstructionScript`
  (`parent.UserConstructionScript`))