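; BP_Book_Rare is a rare book actor that randomizes its identity and look when play begins.
; After running the parent's BeginPlay, it picks a random row from the DT_RareBooks data table and stores it in RareBooksStats.
; That row supplies the candidates for BookMesh, which gets a random small, medium or large scale and a random static mesh.
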(event `self.ReceiveBeginPlay`
  (`parent.ReceiveBeginPlay`)
  ; Set Random Book
  (bind _outrownames (`DataTableFunctionLibrary.GetDataTableRowNames` "/Game/BookStore/Data/RareBooks/DT_RareBooks.DT_RareBooks"))
  (bind _returnvalue (`|GetDataTableRow` "/Game/BookStore/Data/RareBooks/DT_RareBooks.DT_RareBooks" (`KismetArrayLibrary.Array_Random` _outrownames))
    (:`then`
      (bind _output_get (set `self.Rare Books Stats` _returnvalue))
      (bind (_nameofthebook _price _rarity _mesh _smallbooksize _mediumbooksize _largebooksize) (break `/Game/BookStore/Data/RareBooks/S_RareBooks` _output_get))
      ; replace with book mesh
      (`SceneComponent.SetRelativeScale3D` (`self.BookMesh`) (`KismetArrayLibrary.Array_Random` (`|MakeArray` _smallbooksize _mediumbooksize _largebooksize)))
      (`StaticMeshComponent.SetStaticMesh` (`self.BookMesh`) (`KismetArrayLibrary.Array_Random` _mesh)))))

(fn `UserConstructionScript`
  (`parent.UserConstructionScript`))